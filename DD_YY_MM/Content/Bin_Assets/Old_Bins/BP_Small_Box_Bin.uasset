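; BP_Small_Box_Bin is a parcel sorting bin that accepts small box parcels and plays a truck idle sound at its location on BeginPlay.
; Its box overlap ignores the player, destroys small boxes, releases the player's PhysicsHandle, increases the GameMode score and plays a correct sound.
; Crates and normal parcels get flung out by ApplyImpulse, which enables physics and releases the handle, followed by a buzzer.
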(event OnComponentBeginOverlap(Box)
  (params (OverlappedComponent :type Primitive%20Component%20Object%20Reference) (OtherActor :type Actor%20Object%20Reference) (OtherComp :type Primitive%20Component%20Object%20Reference) (OtherBodyIndex :type Integer) (bFromSweep :type Boolean) (SweepResult :type Hit%20Result%20Structure%20%28by%20ref%29))
  (bind _output_get (Variables|Default|SetOther%20Actor OtherActor))
  (Utilities|Casting|CastToBP_Player _output_get
    (:CastFailed
      (Utilities|Casting|CastToBP_Parcel_Small_boxClass (Utilities|GetClass _output_get)
        (:then
          (Actor|DestroyActor (Variables|Default|GetOther%20Actor))
          (bind _asbp_player (Utilities|Casting|CastToBP_Player (Game|Player|GetPlayerPawn 0)))
          (Physics|Components|PhysicsHandle|ReleaseComponent (Variables|/Game/Player_Assets/BP_Player.BP_Player_C|GetPhysicsHandle _asbp_player))
          (bind _asbp_game_mode (Utilities|Casting|CastToBP_GameMode (Game|GetGameMode)))
          (Default|IncreaseScore _asbp_game_mode)
          (Audio|PlaySound2D "/Game/Sound/RawSounds/Correct.Correct"))
        (:CastFailed
          (bind _asbp_parcel_crate (Utilities|Casting|CastToBP_Parcel_Crate OtherActor)
            (:then
              (CallFunction|ApplyImpulse (Variables|/Game/Parcel_Assets/Crate_Parcel/BP_Parcel_Crate.BP_Parcel_Crate_C|GetStaticMesh _asbp_parcel_crate)))
            (:CastFailed
              (bind _asbp_normal_parcel (Utilities|Casting|CastToBP_Normal_Parcel OtherActor))
              (CallFunction|ApplyImpulse (Variables|/Game/Parcel_Assets/NormalParcel/BP_Normal_Parcel.BP_Normal_Parcel_C|GetStaticMesh _asbp_normal_parcel))))
          (Audio|PlaySound2D "/Game/Sound/RawSounds/IncorrectBuzz.IncorrectBuzz"))))))

(event EventBeginPlay
  (Audio|PlaySoundatLocation "/Game/Sound/SoundCues/Truck_Idle.Truck_Idle" (Transformation|GetActorLocation) "0, 0, 0" 1.0 1.0 0.0 0 0 self))

(event Collision|EventActorBeginOverlap
  (params (OtherActor :type Actor%20Object%20Reference)))

(event EventTick
  (params (DeltaSeconds :type Float%20%28single-precision%29)))

(fn ConstructionScript)

(fn ApplyImpulse
  (params (NewParam :type Static%20Mesh%20Component%20Object%20Reference))
  (Physics|SetSimulatePhysics NewParam true)
  (Collision|SetCollisionEnabled NewParam "QueryAndPhysics")
  (Physics|AddImpulse NewParam "0,-3000.000000, 0" "None" true)
  (bind _asbp_player (Utilities|Casting|CastToBP_Player (Game|Player|GetPlayerPawn 0)))
  (Physics|Components|PhysicsHandle|ReleaseComponent (Variables|/Game/Player_Assets/BP_Player.BP_Player_C|GetPhysicsHandle _asbp_player)))