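; Parcel drop-off bin that plays a truck idle sound at its location on BeginPlay.
; Any normal, crate or small-box parcel overlapping its Box increments PlayerOneScore on BP_GameMode and is destroyed.
; Disconnected logic remains for sorting by type: correct parcels score with a sound, while wrong ones get a buzz and are launched out via ApplyImpulse, both releasing the player's physics handle.
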(event OnComponentBeginOverlap(Box)
  (params (OverlappedComponent :type Primitive%20Component%20Object%20Reference) (OtherActor :type Actor%20Object%20Reference) (OtherComp :type Primitive%20Component%20Object%20Reference) (OtherBodyIndex :type Integer) (bFromSweep :type Boolean) (SweepResult :type Hit%20Result%20Structure%20%28by%20ref%29))
  (Utilities|Casting|CastToBP_Normal_Parcel OtherActor
    (:then
      _)
    (:CastFailed
      (Utilities|Casting|CastToBP_Parcel_Crate OtherActor
        (:then
          _)
        (:CastFailed
          (Utilities|Casting|CastToBP_Parcel_Small_box OtherActor)))))
  (bind _asbp_game_mode (Utilities|Casting|CastToBP_GameMode (Game|GetGameMode)))
  (Math|Integer|IncrementInt (Variables|/Game/Maps/Level_0/BP_GameMode.BP_GameMode_C|GetPlayer%20One%20Score _asbp_game_mode)
    (:%20%20
      (Actor|DestroyActor OtherActor))))

(event EventBeginPlay
  (Audio|PlaySoundatLocation "/Game/Sound/SoundCues/Truck_Idle.Truck_Idle" (Transformation|GetActorLocation) "0, 0, 0" 1.0 1.0 0.0 0 0 self))

(fn ConstructionScript)

(fn ApplyImpulse
  (params (NewParam :type Static%20Mesh%20Component%20Object%20Reference))
  (Physics|SetSimulatePhysics NewParam true)
  (Collision|SetCollisionEnabled NewParam "QueryAndPhysics")
  (Physics|AddImpulse NewParam "0,-3000.000000, 0" "None" true)
  (bind _asbp_player (Utilities|Casting|CastToBP_Player (Game|Player|GetPlayerPawn 0)))
  (Physics|Components|PhysicsHandle|ReleaseComponent (Variables|/Game/Player_Assets/BP_Player.BP_Player_C|GetPhysicsHandle _asbp_player)))