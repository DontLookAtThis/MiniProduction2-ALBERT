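; Forklift AI character that charges toward a stored player position with steadily increasing speed.
; While MBMoving is set, Tick ramps CurrentSpeed over time, applies it as max walk speed, prints it for debugging and reissues AIMoveTo toward OldPlayerPos every frame.
; A successful move clears MBMoving; this graph never sets that flag or the target, nor resets the speed.
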(event EventBeginPlay)

(event Collision|EventActorBeginOverlap
  (params (OtherActor :type Actor%20Object%20Reference)))

(event EventTick
  (params (DeltaSeconds :type Float%20%28single-precision%29))
  (if (Variables|Default|Getm_bMoving)
    (bind _output_get (Variables|Default|SetCurrentSpeed (+ (* DeltaSeconds 1e+02) (Variables|Default|GetCurrentSpeed))))
    (Development|PrintString (Utilities|String|ToString(Float) _output_get))
    (Variables|/Script/Engine.CharacterMovementComponent|SetMaxWalkSpeed (Variables|Character|GetCharacterMovement) _output_get)
    (AI|AIMoveTo self (Variables|Default|GetOldPlayerPos) 0 5.0 false
      (:OnSuccess
        (Variables|Default|Setm_bMoving false)))))

(fn ConstructionScript)