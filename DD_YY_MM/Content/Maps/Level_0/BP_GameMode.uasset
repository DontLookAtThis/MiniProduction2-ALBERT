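; Game mode for Level_0 that runs a timed score round with a three-minute countdown.
; BeginPlay spawns a BP_Player, resets timer and score, and starts music plus truck and conveyor sounds.
; Tick uses a one-second Delay to drive UpdateScore, which formats the clock string and, at zero, pauses the game and shows Game_Over_UI with the score.
; IncreaseScore adds points but is not called here, and the GameWon check is empty.
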(event EventBeginPlay
  (Variables|Default|SetDefaultPawnClass "/Game/Player_Assets/BP_Player.BP_Player_C")
  (Class|GameplayStatics|CreatePlayer -1)
  (Actor|Tick|SetActorTickEnabled true)
  (Variables|Default|SetSeconds 0)
  (Variables|Default|SetMinutes 3)
  (Variables|Default|SetTime "03:00")
  (Variables|Default|SetCurrentScore 0)
  (Audio|PlaySound2D "/Game/Sound/RawSounds/BGM_GamePlay.BGM_GamePlay" 0.2)
  (Audio|PlaySoundatLocation "/Game/Sound/RawSounds/Truck_Idle.Truck_Idle" "-1530.000000,-1170.000000,-120.000000" "0, 0, 0" 0.1)
  (Audio|PlaySoundatLocation "/Game/Sound/RawSounds/ConveyerBelt.ConveyerBelt" "-1530.000000,-1170.000000,-120.000000" "0, 0, 0" 0.5 3.0))

(event EventTick
  (params (DeltaSeconds :type Float%20%28single-precision%29))
  (Utilities|FlowControl|Delay 1.0)
  (CallFunction|UpdateScore)
  (if (Variables|Default|GetGameWon)
    _))

(fn ConstructionScript)

(fn IncreaseScore
  (Variables|Default|SetCurrentScore (+ (Variables|Default|GetCurrentScore) 10)))

(fn UpdateScore
  (bind _minutes (Variables|Default|GetMinutes))
  (bind _currentscore (Variables|Default|GetCurrentScore))
  (if (== (Variables|Default|GetSeconds) 0)
    (if (== (Variables|Default|GetMinutes) 0)
      (Game|SetGamePaused true)
      (bind _returnvalue (UserInterface|CreateWidget "/Game/User_Interface/Game_Over_UI.Game_Over_UI_C" (Game|GetPlayerController 0)))
      (UserInterface|Viewport|AddtoViewport _returnvalue 0)
      (Variables|/Game/User_Interface/Game_Over_UI.Game_Over_UI_C|SetScore _returnvalue _currentscore)
      (Default|EndScreen _returnvalue _currentscore)
      (else
        (Math|Integer|DecrementInt (Variables|Default|GetMinutes)
          (:%20%20
            (Variables|Default|SetSeconds 59)
            (if (<= _minutes 9) :!label _label
              (Variables|Default|SetTime (Utilities|String|Append "0" (Utilities|String|ToString(Integer) _minutes) ":"))
              (else
                (Variables|Default|SetTime (Utilities|String|ToString(Integer) _minutes))))
            (if (<= (Variables|Default|GetSeconds) 9)
              (Variables|Default|SetTime (Utilities|String|Append (Variables|Default|GetTime) "0" (Utilities|String|ToString(Integer) (Variables|Default|GetSeconds))))
              (else
                (Variables|Default|SetTime (Utilities|String|Append (Variables|Default|GetTime) (Utilities|String|ToString(Integer) (Variables|Default|GetSeconds))))))
            (return)))))
    (else
      (Math|Integer|DecrementInt (Variables|Default|GetSeconds)
        (:%20%20
          (goto _label))))))