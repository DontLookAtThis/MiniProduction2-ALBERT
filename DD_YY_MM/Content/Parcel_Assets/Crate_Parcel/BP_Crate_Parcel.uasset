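; Crate parcel actor that shows impact effects and breaks apart when its health runs out.
; Tick polls the BoxMechanics health value and, at zero or below, waits briefly before spawning a break emitter and destroying the actor.
; Hard hits above an impulse threshold spawn a hit emitter, ignoring the player, conveyor belts and box components.
; The hit event itself does not change health.
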(event EventTick
  (params (DeltaSeconds :type Float%20%28single-precision%29))
  (if (<= (Variables|/Script/ManagementGame.BoxMechanics|GetiHealth (Variables|Default|GetBoxMechanics)) 0)
    (Utilities|FlowControl|Delay 1.3)
    (Effects|SpawnEmitteratLocation "/Game/VFX/VFX_CrateBreak.VFX_CrateBreak" (Transformation|GetActorLocation) "0, 0, 0" "3.000000,3.000000,3.000000")
    (Actor|DestroyActor)))

(event Collision|EventHit
  (params (MyComp :type Primitive%20Component%20Object%20Reference) (Other :type Actor%20Object%20Reference) (OtherComp :type Primitive%20Component%20Object%20Reference) (bSelfMoved :type Boolean) (HitLocation :type Vector :default "0, 0, 0") (HitNormal :type Vector :default "0, 0, 0") (NormalImpulse :type Vector :default "0, 0, 0") (Hit :type Hit%20Result%20Structure%20%28by%20ref%29))
  (if (> (Math|Vector|VectorLength NormalImpulse) 2e+04)
    (Utilities|Casting|CastToBP_Player Other
      (:CastFailed
        (Utilities|Casting|CastToBP_Conveyor_Belt Other
          (:CastFailed
            (Utilities|Casting|CastToBoxComponent OtherComp
              (:CastFailed
                (Effects|SpawnEmitteratLocation "/Game/VFX/VFX_CrateHit.VFX_CrateHit" (Transformation|GetActorLocation) "0, 0, 0" "6.000000,6.000000,6.000000")))))))))

(fn ConstructionScript)