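; Player character Blueprint that adds a headbutt for shoving other players and making them drop their parcels.
; The HeadButt input, blocked while grabbing, stunned or cooling down, runs a forward box trace with debug drawing.
; A hit player is launched away with upward bias, much harder if stunned, and its ParcelGrabber drops.
; Tick counts down the cooldown and derives the Grabbed flag from the PhysicsHandle.
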(event EventBeginPlay)

(event Collision|EventActorBeginOverlap
  (params (OtherActor :type Actor%20Object%20Reference)))

(event EventTick
  (params (DeltaSeconds :type Float%20%28single-precision%29))
  (if (Variables|Default|GetbCanHeadButt)
    _
    (elif (<= (Variables|Default|GetHeadButtCooldown) 0.0)
      (Variables|Default|SetbCanHeadButt true)
      (Variables|Default|SetHeadButtCooldown 2.0)
      (else
        (Variables|Default|SetHeadButtCooldown (- (Variables|Default|GetHeadButtCooldown) DeltaSeconds)))))
  (Utilities|IsValid (Class|PhysicsHandleComponent|GetGrabbedComponent (Variables|Default|GetPhysicsHandle))
    (:Is%20Valid
      (Variables|Default|SetGrabbed true))
    (:Is%20Not%20Valid
      (Variables|Default|SetGrabbed false))))

(event Input|ActionEvents|InputActionHeadButt
  (params (Key :type Key%20Structure))
  (bind _returnvalue (Transformation|GetActorLocation))
  (:Pressed
    (if (not (or (Variables|Default|GetGrabbed) (Variables|Default|GetbStunned self)))
      (if (Variables|Default|GetbCanHeadButt)
        (Variables|Default|SetbCanHeadButt false)
        (bind (_outhit _returnvalue_2) (Collision|BoxTraceByChannel _returnvalue (+ _returnvalue (* (Transformation|GetActorForwardVector) 2e+02)) "0.000000,50.000000,50.000000" (Transformation|GetActorRotation) "TraceTypeQuery4" false (Utilities|Array|MakeArray self) "ForDuration" true "(R=0.030354,G=0.181177,B=1.000000,A=1.000000)" "(R=0.000000,G=1.000000,B=0.210470,A=1.000000)" (Variables|Default|GetHeadButtCooldown)))
        (if _returnvalue_2
          (bind _asbp_player (Utilities|Casting|CastToBP_Player (.HitActor (Collision|BreakHitResult _outhit))))
          (bind _output_get (Variables|Default|SetPush%20vect (* (Math|Vector|Normalize (+ (- (Transformation|GetActorLocation _asbp_player) (Transformation|GetActorLocation)) "0,0.000000,150.000000")) (Variables|Default|GetPushForce))))
          (if (Variables|/Script/ManagementGame.ManagementGameCharacter|GetbStunned _asbp_player)
            (Variables|Default|SetPush%20vect (* _output_get 4.0)))
          (Character|LaunchCharacter _asbp_player (Variables|Default|GetPush%20vect) true false)
          (Class|ParcelGrabber|DropAction (Variables|BP_Player_C|GetParcelGrabber _asbp_player)))))))

(fn ConstructionScript)